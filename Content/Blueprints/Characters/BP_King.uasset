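; BP_King is a player-controlled character Blueprint with Enhanced Input set up and placeholder responses to jump and move input.
; On BeginPlay it casts its controller to PlayerController and adds the IMC_Character mapping context to the local player subsystem.
; The Started events of IA_Jump and IA_Move only print debug strings, so no movement or jump logic runs in this graph.
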(event `self.ReceiveBeginPlay`
  (`parent.ReceiveBeginPlay`)
  (bind _asplayer_controller (cast `PlayerController` (`self.GetController`)))
  (`EnhancedInputSubsystemInterface.AddMappingContext` (pcsubsystem `EnhancedInputLocalPlayerSubsystem` _asplayer_controller) "/Game/Inputs/IMC_Character.IMC_Character" 0 (struct)))

(event `EnhancedInput|/Game/Inputs/Actions/IA_Jump`
  (params (ActionValue :type Boolean) (ElapsedSeconds :type "Float (double-precision)") (TriggeredSeconds :type "Float (double-precision)") (InputAction :type "InputAction Object Reference" :default "/Game/Inputs/Actions/IA_Jump.IA_Jump"))
  (:`Started`
    (`KismetSystemLibrary.PrintString` "Jump!")))

(event `EnhancedInput|/Game/Inputs/Actions/IA_Move`
  (params (ActionValue :type "Float (double-precision)") (ElapsedSeconds :type "Float (double-precision)") (TriggeredSeconds :type "Float (double-precision)") (InputAction :type "InputAction Object Reference" :default "/Game/Inputs/Actions/IA_Move.IA_Move"))
  (:`Started`
    (`KismetSystemLibrary.PrintString` "Move!")))

(fn `UserConstructionScript`
  (`parent.UserConstructionScript`))