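; BP_King is the player character for a side-scrolling platformer, moving along X with Enhanced Input and facing its direction of travel.
; Retriggerable delays drive jump buffering and coyote time, the latter feeding the CanJumpInternal override.
; While airborne, a downward foot trace toggles capsule collision so thin ledges block only on descent.
; Falling onto a BP_Pig kills it and bounces; other pig contact triggers death with camera detach, sound and shake.
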(event `self.ReceiveBeginPlay`
  (`parent.ReceiveBeginPlay`)
  (bind _asplayer_controller (cast `PlayerController` (`self.GetController`)))
  (`EnhancedInputSubsystemInterface.AddMappingContext` (pcsubsystem `EnhancedInputLocalPlayerSubsystem` _asplayer_controller) "/Game/Inputs/IMC_Character.IMC_Character" 0 (struct)))

(event `self.ReceiveTick`
  (params (DeltaSeconds :type "Float (single-precision)"))
  (`parent.ReceiveTick` DeltaSeconds)
  (`self.UpateControllerRotation`)
  (`self.TraceLedgeThin`)
  (if (and (`self.CanJump`) (`self.IsJumpBuffering`))
    (`self.Jump`)))

(event `EnhancedInput|/Game/Inputs/Actions/IA_Jump`
  (params (ActionValue :type Boolean) (ElapsedSeconds :type "Float (double-precision)") (TriggeredSeconds :type "Float (double-precision)") (InputAction :type "InputAction Object Reference" :default "/Game/Inputs/Actions/IA_Jump.IA_Jump"))
  (:`Started`
    (if (`self.CanJump`)
      (`self.Jump`)
      (else
        (set `self.IsJumpBuffering` true)
        (`KismetSystemLibrary.RetriggerableDelay` (`self.JumpBufferDuration`))
        (set `self.IsJumpBuffering` false))))
  (:`Completed`
    (`self.StopJumping`)))

(event `EnhancedInput|/Game/Inputs/Actions/IA_Move`
  (params (ActionValue :type "Float (double-precision)") (ElapsedSeconds :type "Float (double-precision)") (TriggeredSeconds :type "Float (double-precision)") (InputAction :type "InputAction Object Reference" :default "/Game/Inputs/Actions/IA_Move.IA_Move"))
  (:`Triggered`
    (`self.AddMovementInput` (1.0 0.0 0.0) ActionValue)))

(event `self.CapsuleComponent.OnComponentBeginOverlap`
  (params (OverlappedComponent :type "PrimitiveComponent Object Reference") (OtherActor :type "Actor Object Reference") (OtherComp :type "PrimitiveComponent Object Reference") (OtherBodyIndex :type Integer) (bFromSweep :type Boolean) (SweepResult :type "HitResult Structure (by ref)"))
  (bind (_returnvalue_x _returnvalue_y _returnvalue_z) (`KismetMathLibrary.BreakVector` (`self.GetVelocity`)))
  (bind _asbp_pig (cast `/Game/Blueprints/Characters/Pig/BP_Pig` OtherActor))
  (if (and (`NavMovementComponent.IsFalling` (`self.CharacterMovement`)) (< _returnvalue_z 0.0))
    (`self.Death` _asbp_pig)
    (`self.LaunchCharacter` (`KismetMathLibrary.MakeVector` 0.0 0.0 (`self.BounceLaunch`)) false true)
    (else
      (`self.Death`))))

(event `self.Death`
  (`parent.Death`)
  (bind _asplayer_controller (cast `PlayerController` (`self.GetController`)))
  (`EnhancedInputSubsystemInterface.RemoveMappingContext` (pcsubsystem `EnhancedInputLocalPlayerSubsystem` _asplayer_controller) "/Game/Inputs/IMC_Character.IMC_Character" (struct))
  (`SceneComponent.K2_DetachFromComponent` (`self.SpringArm`) "KeepWorld" "KeepRelative" "KeepRelative" true)
  (`GameplayStatics.PlaySound2D` "/Game/Sounds/King/Defeated/S_Defeated_Cue.S_Defeated_Cue" 1.0 1.0 0.0 null null)
  (`GameplayStatics.PlayWorldCameraShake` "/Game/Blueprints/Camera/BP_CameraShake.BP_CameraShake_C" (`self.K2_GetActorLocation`) 0.0 10000.0 0.0))

(event `self.OnWalkingOffLedge`
  (params (PreviousFloorImpactNormal :type "Vector Structure (by ref)") (PreviousFloorContactNormal :type "Vector Structure (by ref)") (PreviousLocation :type "Vector Structure (by ref)") (TimeDelta :type "Float (single-precision)"))
  (set `self.IsCoyoteTime` true)
  (`KismetSystemLibrary.RetriggerableDelay` (`self.CoyoteTimeDuratioon`))
  (set `self.IsCoyoteTime` false))

(fn `CanJumpInternal`
  (returns (ReturnValue :type Boolean))
  (bind _returnvalue (`parent.CanJumpInternal`))
  (return (or _returnvalue (`self.IsCoyoteTime`))))

(fn `TraceLedgeThin`
  (bind (_returnvalue_x _returnvalue_y _returnvalue_z) (`KismetMathLibrary.BreakVector` (`self.GetVelocity`)))
  (bind _returnvalue (`SceneComponent.K2_GetComponentLocation` (`self.Foot`)))
  (if (`NavMovementComponent.IsFalling` (`self.CharacterMovement`))
    (bind (_outhit _returnvalue_2) (`KismetSystemLibrary.LineTraceSingleForObjects` :`Start` _returnvalue :`End` (+ _returnvalue (* (`KismetMathLibrary.Vector_Down`) (`self.LedgeTraceDistance`))) :`ObjectTypes` (`|MakeArray` "ObjectTypeQuery7" :!type "EObjectTypeQuery Enum") :`DrawDebugType` "ForOneFrame"))
    (if (and _returnvalue_2 (< _returnvalue_z 0.0))
      (`PrimitiveComponent.SetCollisionResponseToChannel` (`self.CapsuleComponent`) "ECC_GameTraceChannel1" "ECR_Block")
      (else
        (`PrimitiveComponent.SetCollisionResponseToChannel` (`self.CapsuleComponent`) "ECC_GameTraceChannel1" "ECR_Overlap")))))

(fn `UpateControllerRotation`
  (bind _returnvalue (`self.GetController`))
  (bind _returnvalue_2 (`self.GetController`))
  (bind _velocity_x (`KismetMathLibrary.BreakVector` (`MovementComponent.Velocity` (`self.CharacterMovement`))))
  (`/Engine/EditorBlueprintResources/StandardMacros.CompareFloat` _velocity_x
    (:`>`
      (`/Engine/EditorBlueprintResources/StandardMacros.IsValid` _returnvalue_2
        (:`Is Valid`
          (`Controller.SetControlRotation` _returnvalue_2 (`KismetMathLibrary.MakeRotator` 0.0)))))
    (:`<`
      (`/Engine/EditorBlueprintResources/StandardMacros.IsValid` _returnvalue
        (:`Is Valid`
          (`Controller.SetControlRotation` _returnvalue (`KismetMathLibrary.MakeRotator` 0.0 0.0 180.0)))))))

(fn `UserConstructionScript`
  (`parent.UserConstructionScript`))