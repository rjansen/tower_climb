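; Character Blueprint that handles a one-time death sequence, with no other active logic.
; The Death event sets IsDead to block repeats, disables capsule collision and calls LaunchOnDeath.
; LaunchOnDeath releases the movement plane constraint and launches the character along world up and right vectors scaled by tunable strengths, overriding current velocity.
; The anim instance then jumps straight to its Death node.
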(event `Death`
  (if (not (`self.IsDead`))
    (set `self.IsDead` true)
    (`PrimitiveComponent.SetCollisionEnabled` (`self.CapsuleComponent`) "NoCollision")
    (`self.LaunchOnDeath`)
    (`PaperZDAnimInstance.JumpToNode` (`self.AnimInstance`) "Death" "None")))

(fn `LaunchOnDeath`
  (`MovementComponent.SetPlaneConstraintEnabled` (`self.CharacterMovement`) false)
  (`self.LaunchCharacter` (+ (* (`KismetMathLibrary.Vector_Up`) (`self.LaunchUp`)) (* (`KismetMathLibrary.Vector_Right`) (`self.LaunchRight`))) true true))

(fn `UserConstructionScript`)